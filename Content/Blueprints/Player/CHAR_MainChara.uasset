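; Player character Blueprint that lets the player shove special cubes with the Interact input.
; On press, it line-traces a short distance from the actor along the controller's rotation, ignoring every StaticMeshActor and drawing debug lines.
; A hit BP_CubeThatDoesNotKillYou or its Sideways variant receives a strong impulse along a fixed world axis specific to that type, regardless of facing.
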(event Input|EnhancedActionEvents|EnhancedInputActionIA_Interact
  (params (ActionValue :type Boolean) (ElapsedSeconds :type Float%20%28double-precision%29) (TriggeredSeconds :type Float%20%28double-precision%29) (InputAction :type Input%20Action%20Object%20Reference :default "/Game/Input/Actions/IA_Interact.IA_Interact"))
  (bind _returnvalue (Transformation|GetActorLocation))
  (:Started
    (bind _outactors (Actor|GetAllActorsOfClass "/Script/Engine.StaticMeshActor"))
    (bind _outhit (Collision|LineTraceByChannel _returnvalue (+ _returnvalue (Math|Vector|RotateVector (Math|Vector|MakeVector 1.4e+02 0.0 0.0) (Transformation|GetWorldRotation (Variables|/Script/Engine.Actor|GetRootComponent (Pawn|GetController))))) "TraceTypeQuery1" false _outactors "ForDuration"))
    (bind _asbp_cube_that_does_not_kill_you (Utilities|Casting|CastToBP_CubeThatDoesNotKillYou (.hitactor _outhit))
      (:then
        (Physics|AddImpulse (Variables|/Game/Blueprints/Obstacles/BP_CubeThatDoesNotKillYou.BP_CubeThatDoesNotKillYou_C|GetStaticMesh _asbp_cube_that_does_not_kill_you) "200000.000000,0.000000,0.000000" "None" false))
      (:CastFailed
        (bind _asbp_cube_that_does_not_kill_you_sideways (Utilities|Casting|CastToBP_CubeThatDoesNotKillYouSideways (.hitactor _outhit)))
        (Physics|AddImpulse (Variables|/Game/Blueprints/Obstacles/BP_CubeThatDoesNotKillYouSideways.BP_CubeThatDoesNotKillYouSideways_C|GetStaticMesh _asbp_cube_that_does_not_kill_you_sideways) "0.000000,-200000.000000,0.000000" "None" false)))))

(event EventBeginPlay)

(event Collision|EventActorBeginOverlap
  (params (OtherActor :type Actor%20Object%20Reference)))

(event EventTick
  (params (DeltaSeconds :type Float%20%28single-precision%29)))

(fn ConstructionScript)