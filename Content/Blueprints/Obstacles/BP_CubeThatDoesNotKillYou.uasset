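; BP_CubeThatDoesNotKillYou is an obstacle cube that clears BP_GoodbyeWall actors and can open up a BP_DeathForcefield.
; Overlapping a BP_GoodbyeWall destroys both that wall and the cube.
; If no BP_CubeThatDoesNotKillYouSideways actors exist at that moment, it also destroys every remaining GoodbyeWall and the DeathForcefield nearest to itself.
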(event EventBeginPlay)

(event Collision|EventActorBeginOverlap
  (params (OtherActor :type Actor%20Object%20Reference))
  (bind _asbp_goodbye_wall (Utilities|Casting|CastToBP_GoodbyeWall OtherActor))
  (Actor|DestroyActor _asbp_goodbye_wall)
  (bind _outactors (Actor|GetAllActorsOfClass "/Game/Blueprints/Obstacles/BP_CubeThatDoesNotKillYouSideways.BP_CubeThatDoesNotKillYouSideways_C"))
  (if (== (Utilities|Array|Length _outactors) 0)
    (bind _outactors_2 (Actor|GetAllActorsOfClass "/Game/Blueprints/Obstacles/BP_GoodbyeWall.BP_GoodbyeWall_C"))
    (for _array_element _outactors_2
      (Actor|DestroyActor _array_element))
    (bind _outactors_3 (Actor|GetAllActorsOfClass "/Game/Blueprints/Obstacles/BP_DeathForcefield.BP_DeathForcefield_C"))
    (Actor|DestroyActor (.ReturnValue (Actor|FindNearestActor (Transformation|GetActorLocation) _outactors_3))))
  (Actor|DestroyActor))

(event EventTick
  (params (DeltaSeconds :type Float%20%28single-precision%29)))

(fn ConstructionScript)